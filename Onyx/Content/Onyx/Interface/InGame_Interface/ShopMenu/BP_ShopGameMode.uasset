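; Game mode for the shop level, the timed phase that leads into the next arena round.
; On BeginPlay it points player 0's view at a camera actor, caches BP_GameInstance and adds the default input mapping.
; A container widget receives the two-player, two-team or four-player shop overlay based on GameInstance counts, and a second, empty container follows.
; A one-minute timer fires EndRound, which increments the stored round and opens Arena1.
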(event Custom|AddWidgetOverlay
  (bind _returnvalue (UserInterface|CreateWidget "/Game/Onyx/Interface/WBP_ContainerWidget.WBP_ContainerWidget_C"))
  (Variables|Default|SetUserInterface _returnvalue)
  (UserInterface|Viewport|AddtoViewport _returnvalue 0)
  (if (== (Variables|/Game/Onyx/GameCore/BP_GameInstance.BP_GameInstance_C|GetNumPlayers (Variables|Default|GetGame%20Instance)) 2)
    (Default|PushMenuOverlay (Variables|Default|GetUserInterface) "/Game/Onyx/Interface/InGame_Interface/ShopMenu/WBP_Shop_Interface_2_Players.WBP_Shop_Interface_2_Players_C")
    (elif (== (Variables|/Game/Onyx/GameCore/BP_GameInstance.BP_GameInstance_C|GetNumTeams (Variables|Default|GetGame%20Instance)) 2)
      (Default|PushMenuOverlay (Variables|Default|GetUserInterface) "/Game/Onyx/Interface/InGame_Interface/ShopMenu/WBP_Shop_Interface_2_Teams.WBP_Shop_Interface_2_Teams_C")
      (else
        (Default|PushMenuOverlay (Variables|Default|GetUserInterface) "/Game/Onyx/Interface/InGame_Interface/ShopMenu/WBP_Shop_Interface_4_Players.WBP_Shop_Interface_4_Players_C")))))

(event Custom|EndRound
  (bind _game_instance (Variables|Default|GetGame%20Instance))
  (Utilities|Time|ClearandInvalidateTimerbyHandle (stale EventBeginPlay _returnvalue_2))
  (bind _result (Math|Integer|IncrementInt (Variables|/Game/Onyx/GameCore/BP_GameInstance.BP_GameInstance_C|GetRound _game_instance))
    (:%20%20
      (Variables|/Game/Onyx/GameCore/BP_GameInstance.BP_GameInstance_C|SetRound _game_instance _result)
      (Game|OpenLevel(byObjectReference) "/Game/Onyx/Levels/Maps/Arena1.Arena1"))))

(event EventBeginPlay
  (bind _returnvalue (Actor|GetActorOfClass "/Script/Engine.CameraActor"))
  (Game|Player|SetViewTargetwithBlend (Game|GetPlayerController 0) _returnvalue 0.0 "VTBlend_Linear" 0.0 false)
  (bind _asbp_game_instance (Utilities|Casting|CastToBP_GameInstance (Game|GetGameInstance)))
  (Variables|Default|SetGame%20Instance _asbp_game_instance)
  (CallFunction|AddWidgetOverlay)
  (bind _returnvalue_2 (Utilities|Time|SetTimerbyEvent (delegate Custom|EndRound) 6e+01))
  (Input|AddMappingContext (PlayerController|LocalPlayerSubsystems|GetEnhancedInputLocalPlayerSubsystem (Game|GetPlayerController 0)) "/Game/Onyx/Input/IMC_Default.IMC_Default" 0 "(bIgnoreAllPressedKeysUntilRelease=True,bForceImmediately=False,bNotifyUserSettings=False)")
  (bind _returnvalue_3 (UserInterface|CreateWidget "/Game/Onyx/Interface/WBP_ContainerWidget.WBP_ContainerWidget_C"))
  (Variables|Default|SetOverlay _returnvalue_3)
  (UserInterface|Viewport|AddtoViewport _returnvalue_3 0))

(fn ConstructionScript)