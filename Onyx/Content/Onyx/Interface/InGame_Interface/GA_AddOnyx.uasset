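; GA_AddOnyx is a Gameplay Ability that grants Onyx to its owner.
; On activation it commits, then builds a GE_AddOnyx spec and passes the amount through the Data.OnyxReceive SetByCaller tag.
; The amount is OnyxReceive plus a bonus scaled by the ratio of two of the owner's attribute values.
; It applies the spec to the owner's Ability System Component and ends, or ends immediately if the commit fails.
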(event Ability|EventActivateAbility
  (bind _returnvalue (Ability|GetOwningActorfromActorInfo))
  (bind _onyxreceive (Variables|Default|GetOnyxReceive))
  (bind _returnvalue_2 (Ability|GetAbilitySystemComponent _returnvalue))
  (bind _returnvalue_3 (Ability|CommitAbility))
  (if _returnvalue_3
    (bind _returnvalue_4 (Ability|GameplayEffect|AssignTagSetbyCallerMagnitude (Ability|MakeOutgoingGameplayEffectSpec "/Game/Onyx/Effects/GE_AddOnyx.GE_AddOnyx_C") "(TagName=\"Data.OnyxReceive\")" (+ _onyxreceive (* _onyxreceive (/ (.ReturnValue (Class|AbilitySystemComponent|GetGameplayAttributeValue _returnvalue_2 "(AttributeName=\"Health\",Attribute=/Script/Onyx.OnyxAttributeSet:Health,AttributeOwner=\"/Script/CoreUObject.Class'/Script/Onyx.OnyxAttributeSet'\")")) (.ReturnValue (Class|AbilitySystemComponent|GetGameplayAttributeValue _returnvalue_2 "(AttributeName=\"MaxHealth\",Attribute=/Script/Onyx.OnyxAttributeSet:MaxHealth,AttributeOwner=\"/Script/CoreUObject.Class'/Script/Onyx.OnyxAttributeSet'\")")))))))
    (GameplayEffects|ApplyGameplayEffectSpecToSelf _returnvalue_2 _returnvalue_4)
    (Ability|EndAbility)
    (else
      (Ability|EndAbility))))

(event Ability|EventOnEndAbility
  (params (bWasCancelled :type Boolean)))