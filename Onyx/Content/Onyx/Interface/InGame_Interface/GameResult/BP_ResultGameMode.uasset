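; Game mode for the match result screen, showing each player's chosen fighter on a fixed camera with a result menu.
; BeginPlay views through the level's CameraActor, pushes a two-player, two-team or four-player result widget based on GameInstance, and adds input mapping.
; Placed BP_Fighter_SelectMenu actors are paired by array index with player selections to show mesh, skin and montage.
; Actors beyond the player count are hidden.
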(event Custom|AddWidgetOverlay
  (bind _returnvalue (UserInterface|CreateWidget "/Game/Onyx/Interface/WBP_ContainerWidget.WBP_ContainerWidget_C"))
  (Variables|Default|SetWidgetOverlay _returnvalue)
  (UserInterface|Viewport|AddtoViewport _returnvalue 0)
  (if (== (Variables|/Game/Onyx/GameCore/BP_GameInstance.BP_GameInstance_C|GetNumPlayers (Variables|Default|GetGameInstance)) 2)
    (Default|PushMenuOverlay (Variables|Default|GetWidgetOverlay) "/Game/Onyx/Interface/InGame_Interface/GameResult/WBP_Result_Interface_2_Players.WBP_Result_Interface_2_Players_C")
    (elif (== (Variables|/Game/Onyx/GameCore/BP_GameInstance.BP_GameInstance_C|GetNumTeams (Variables|Default|GetGameInstance)) 2)
      (Default|PushMenuOverlay (Variables|Default|GetWidgetOverlay) "/Game/Onyx/Interface/InGame_Interface/GameResult/WBP_Result_Interface_2_Teams.WBP_Result_Interface_2_Teams_C")
      (else
        (Default|PushMenuOverlay (Variables|Default|GetWidgetOverlay) "/Game/Onyx/Interface/InGame_Interface/GameResult/WBP_Result_Interface_4_Players.WBP_Result_Interface_4_Players_C")))))

(event EventBeginPlay
  (bind _returnvalue (Actor|GetActorOfClass "/Script/Engine.CameraActor"))
  (Game|Player|SetViewTargetwithBlend (Game|GetPlayerController 0) _returnvalue 0.0 "VTBlend_Linear" 0.0 false)
  (bind _asbp_game_instance (Utilities|Casting|CastToBP_GameInstance (Game|GetGameInstance)))
  (Variables|Default|SetGameInstance _asbp_game_instance)
  (CallFunction|AddWidgetOverlay)
  (Input|AddMappingContext (PlayerController|LocalPlayerSubsystems|GetEnhancedInputLocalPlayerSubsystem (Game|GetPlayerController 0)) "/Game/Onyx/Input/IMC_Default.IMC_Default" 0 "(bIgnoreAllPressedKeysUntilRelease=True,bForceImmediately=False,bNotifyUserSettings=False)")
  (bind _outactors (Actor|GetAllActorsOfClass "/Game/Onyx/Interface/SelectFighter/BP_Fighter_SelectMenu.BP_Fighter_SelectMenu_C"))
  (Variables|Default|SetFighters _outactors)
  (for (_array_element _array_index) (Variables|Default|GetFighters)
    (switch name (.fighterselected (Utilities|Array|Get(acopy) (Variables|/Game/Onyx/GameCore/BP_GameInstance.BP_GameInstance_C|GetPlayerSelection (Variables|Default|GetGameInstance)) _array_index))
      (:Countess
        (Variables|Default|SetFighterSelected 0))
      (:Grim
        (Variables|Default|SetFighterSelected 1))
      (:Grux
        (Variables|Default|SetFighterSelected 2))
      (:Iggy
        (Variables|Default|SetFighterSelected 3))
      (:Khaimera
        (Variables|Default|SetFighterSelected 4))
      (:Phase
        (Variables|Default|SetFighterSelected 5))
      (:Sevarog
        (Variables|Default|SetFighterSelected 6))
      (:Sparrow
        (Variables|Default|SetFighterSelected 7))
      (:Terra
        (Variables|Default|SetFighterSelected 8)))
    (Rendering|SetVisibility (.SkeletalMeshComponent (Utilities|Struct|BreakF_Fighters (Utilities|Array|Get(acopy) (Variables|/Game/Onyx/Interface/SelectFighter/BP_Fighter_SelectMenu.BP_Fighter_SelectMenu_C|GetFightersStructureArray _array_element) (Variables|Default|GetFighterSelected)))) true false)
    (Default|ChangeMesh _array_element (.SkeletalMeshComponent (Utilities|Struct|BreakF_Fighters (Utilities|Array|Get(acopy) (Variables|/Game/Onyx/Interface/SelectFighter/BP_Fighter_SelectMenu.BP_Fighter_SelectMenu_C|GetFightersStructureArray _array_element) (Variables|Default|GetFighterSelected)))) (Utilities|Array|Get(acopy) (.skeletalmesh (Utilities|Array|Get(acopy) (Variables|/Game/Onyx/Interface/SelectFighter/BP_Fighter_SelectMenu.BP_Fighter_SelectMenu_C|GetSkinsStructureArray _array_element) (Variables|Default|GetFighterSelected))) (.skinselected (Utilities|Array|Get(acopy) (Variables|/Game/Onyx/GameCore/BP_GameInstance.BP_GameInstance_C|GetPlayerSelection (Variables|Default|GetGameInstance)) _array_index))))
    (Animation|Montage|PlayMontage (.SkeletalMeshComponent (Utilities|Struct|BreakF_Fighters (Utilities|Array|Get(acopy) (Variables|/Game/Onyx/Interface/SelectFighter/BP_Fighter_SelectMenu.BP_Fighter_SelectMenu_C|GetFightersStructureArray _array_element) (Variables|Default|GetFighterSelected)))) (.AnimMontage (Utilities|Struct|BreakF_Fighters (Utilities|Array|Get(acopy) (Variables|/Game/Onyx/Interface/SelectFighter/BP_Fighter_SelectMenu.BP_Fighter_SelectMenu_C|GetFightersStructureArray _array_element) (Variables|Default|GetFighterSelected))))))
  (for (_array_element_2 _array_index_2) (Variables|Default|GetFighters)
    (if (>= _array_index_2 (Variables|/Game/Onyx/GameCore/BP_GameInstance.BP_GameInstance_C|GetNumPlayers (Variables|Default|GetGameInstance)))
      (Rendering|SetActorHiddenInGame _array_element_2 true))))

(fn ConstructionScript)