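; BP_SelectFighterGameModeAI sets up the fighter selection screen.
; On BeginPlay it points the first player's view at the level camera, resets the game through BP_GameInstance and adds a container widget to the viewport.
; The container gets the two-player selection menu, or the four-player menu for any other player count.
; It then creates the additional local players and gives each player the default Enhanced Input mapping context.
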(event Custom|AddWidgetOverlay
  (bind _returnvalue (UserInterface|CreateWidget "/Game/Onyx/Interface/WBP_ContainerWidget.WBP_ContainerWidget_C"))
  (Variables|Default|SetWidgetOverlay _returnvalue)
  (UserInterface|Viewport|AddtoViewport _returnvalue 0)
  (if (== (Variables|/Game/Onyx/GameCore/BP_GameInstance.BP_GameInstance_C|GetNumPlayers (Variables|Default|GetGameInstance)) 2)
    (Default|PushMenuOverlay (Variables|Default|GetWidgetOverlay) "/Game/Onyx/Interface/SelectFighter/WBP_SelectFighter.WBP_SelectFighter_C")
    (else
      (Default|PushMenuOverlay (Variables|Default|GetWidgetOverlay) "/Game/Onyx/Interface/SelectFighter/WBP_SelectFighter_4Players.WBP_SelectFighter_4Players_C"))))

(event EventBeginPlay
  (bind _returnvalue (Actor|GetActorOfClass "/Script/Engine.CameraActor"))
  (Game|Player|SetViewTargetwithBlend (Game|GetPlayerController 0) _returnvalue 0.0 "VTBlend_Linear" 0.0 false)
  (bind _asbp_game_instance (Utilities|Casting|CastToBP_GameInstance (Game|GetGameInstance)))
  (bind _output_get (Variables|Default|SetGameInstance _asbp_game_instance))
  (Default|ResetGame _output_get)
  (CallFunction|AddWidgetOverlay)
  (for _index (range 1 (- (Variables|/Game/Onyx/GameCore/BP_GameInstance.BP_GameInstance_C|GetNumPlayers (Variables|Default|GetGameInstance)) 1))
    (Class|GameplayStatics|CreatePlayer _index))
  (for _index_2 (range 0 (- (Variables|/Game/Onyx/GameCore/BP_GameInstance.BP_GameInstance_C|GetNumPlayers (Variables|Default|GetGameInstance)) 1))
    (Input|AddMappingContext (PlayerController|LocalPlayerSubsystems|GetEnhancedInputLocalPlayerSubsystem (Class|GameplayStatics|GetPlayerControllerfromID _index_2)) "/Game/Onyx/Input/IMC_Default.IMC_Default" 0 "(bIgnoreAllPressedKeysUntilRelease=True,bForceImmediately=False,bNotifyUserSettings=False)")))

(fn ConstructionScript)