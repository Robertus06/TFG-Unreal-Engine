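; Player controller for the shop that drives its pause menu through Enhanced Input actions.
; The pause action toggles the game's paused state, removing the active menu overlay widget or pushing the shop pause menu when none is active.
; The decline action swaps any other active menu back to the shop pause menu, acting as a back button.
; Overlays are reached through the shop game mode cached on BeginPlay.
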(event Input|EnhancedActionEvents|EnhancedInputActionIA_Pause
  (params (ActionValue :type Boolean) (ElapsedSeconds :type Float%20%28double-precision%29) (TriggeredSeconds :type Float%20%28double-precision%29) (InputAction :type Input%20Action%20Object%20Reference :default "/Game/Onyx/Input/Actions/IA_Pause.IA_Pause"))
  (bind _gamemode (Variables|Default|GetGameMode))
  (bind _overlay (Variables|/Game/Onyx/Interface/InGame_Interface/ShopMenu/BP_ShopGameMode.BP_ShopGameMode_C|GetOverlay _gamemode))
  (bind _menuoverlay (Variables|/Game/Onyx/Interface/WBP_ContainerWidget.WBP_ContainerWidget_C|GetMenuOverlay _overlay))
  (bind _returnvalue (Class|CommonActivatableWidgetContainerBase|GetActiveWidget _menuoverlay))
  (:Completed
    (Utilities|IsValid _returnvalue
      (:Is%20Valid
        (Default|RemoveMenuOverlay _overlay _returnvalue)
        (Game|SetGamePaused false))
      (:Is%20Not%20Valid
        (Default|PushMenuOverlay _overlay "/Game/Onyx/Interface/PauseMenu/WBP_PauseMenu_Shop.WBP_PauseMenu_Shop_C")
        (Game|SetGamePaused true)))))

(event Input|EnhancedActionEvents|EnhancedInputActionIA_NavMenu_Decline
  (params (ActionValue :type Boolean) (ElapsedSeconds :type Float%20%28double-precision%29) (TriggeredSeconds :type Float%20%28double-precision%29) (InputAction :type Input%20Action%20Object%20Reference :default "/Game/Onyx/Input/Actions/IA_NavMenu_Decline.IA_NavMenu_Decline"))
  (bind _gamemode (Variables|Default|GetGameMode))
  (bind _overlay (Variables|/Game/Onyx/Interface/InGame_Interface/ShopMenu/BP_ShopGameMode.BP_ShopGameMode_C|GetOverlay _gamemode))
  (bind _menuoverlay (Variables|/Game/Onyx/Interface/WBP_ContainerWidget.WBP_ContainerWidget_C|GetMenuOverlay _overlay))
  (bind _returnvalue (Class|CommonActivatableWidgetContainerBase|GetActiveWidget _menuoverlay))
  (:Completed
    (Utilities|IsValid _returnvalue
      (:Is%20Valid
        (Utilities|Casting|CastToWBP_PauseMenu_Shop _returnvalue
          (:CastFailed
            (Default|RemoveMenuOverlay _overlay _returnvalue)
            (Default|PushMenuOverlay _overlay "/Game/Onyx/Interface/PauseMenu/WBP_PauseMenu_Shop.WBP_PauseMenu_Shop_C")))))))

(event EventBeginPlay
  (bind _asbp_shop_game_mode (Utilities|Casting|CastToBP_ShopGameMode (Game|GetGameMode)))
  (Variables|Default|SetGameMode _asbp_shop_game_mode)
  (bind _asbp_game_instance (Utilities|Casting|CastToBP_GameInstance (Game|GetGameInstance)))
  (Variables|Default|SetGameInstance _asbp_game_instance))

(event EventTick
  (params (DeltaSeconds :type Float%20%28single-precision%29)))

(fn ConstructionScript)