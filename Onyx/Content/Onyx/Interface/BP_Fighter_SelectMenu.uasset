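; BP_Fighter_SelectMenu is a fighter-selection display actor that cycles through nine skeletal mesh components.
; On BeginPlay it enables input from player controller 0 so it can receive the T key directly.
; Each T press steps a looping, non-random MultiGate that hides the current mesh and shows the next, wrapping from the ninth back to the first.
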(event EventBeginPlay
  (Input|EnableInput (Game|GetPlayerController 0)))

(event Collision|EventActorBeginOverlap
  (params (OtherActor :type Actor%20Object%20Reference)))

(event EventTick
  (params (DeltaSeconds :type Float%20%28single-precision%29)))

(event Input|KeyboardEvents|T
  (params (Key :type Key%20Structure :default "None"))
  (:Pressed
    (Utilities|FlowControl|MultiGate false true -1
      (:Out%200
        (Rendering|SetVisibility (Variables|Default|GetSkeletalMesh1) false false)
        (Rendering|SetVisibility (Variables|Default|GetSkeletalMesh2) true false))
      (:Out%201
        (Rendering|SetVisibility (Variables|Default|GetSkeletalMesh2) false false)
        (Rendering|SetVisibility (Variables|Default|GetSkeletalMesh3) true false))
      (:Out%202
        (Rendering|SetVisibility (Variables|Default|GetSkeletalMesh3) false false)
        (Rendering|SetVisibility (Variables|Default|GetSkeletalMesh4) true false))
      (:Out%203
        (Rendering|SetVisibility (Variables|Default|GetSkeletalMesh4) false false)
        (Rendering|SetVisibility (Variables|Default|GetSkeletalMesh5) true false))
      (:Out%204
        (Rendering|SetVisibility (Variables|Default|GetSkeletalMesh5) false false)
        (Rendering|SetVisibility (Variables|Default|GetSkeletalMesh6) true false))
      (:Out%205
        (Rendering|SetVisibility (Variables|Default|GetSkeletalMesh6) false false)
        (Rendering|SetVisibility (Variables|Default|GetSkeletalMesh7) true false))
      (:Out%206
        (Rendering|SetVisibility (Variables|Default|GetSkeletalMesh7) false false)
        (Rendering|SetVisibility (Variables|Default|GetSkeletalMesh8) true false))
      (:Out%207
        (Rendering|SetVisibility (Variables|Default|GetSkeletalMesh8) false false)
        (Rendering|SetVisibility (Variables|Default|GetSkeletalMesh9) true false))
      (:Out%208
        (Rendering|SetVisibility (Variables|Default|GetSkeletalMesh9) false false)
        (Rendering|SetVisibility (Variables|Default|GetSkeletalMesh1) true false)))))

(fn ConstructionScript)