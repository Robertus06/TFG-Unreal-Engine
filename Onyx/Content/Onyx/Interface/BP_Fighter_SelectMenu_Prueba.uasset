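; Fighter select menu preview Blueprint that displays the hovered fighter's animated skeletal mesh.
; The construction script reads every row of FightersDataTable, creates a hidden skeletal mesh component with that fighter's mesh and Anim Blueprint, and stores it in StructureArray.
; SelectFighter takes a hovered index, hides all fighter meshes, reveals the matching one and plays its montage.
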(event Custom|SelectFighter
  (params (FighterHovered :type Integer))
  (bind _structurearray (Variables|Default|GetStructureArray))
  (bind _output (Utilities|Array|Get(acopy) _structurearray FighterHovered))
  (bind (_skeletalmesh _skeletalmeshcomponent _animblueprint _animmontage) (Utilities|Struct|BreakF_Fighters _output))
  (for _array_element _structurearray
    (Rendering|SetVisibility (.skeletalmeshcomponent _array_element) false false))
  (Rendering|SetVisibility _skeletalmeshcomponent true false)
  (Animation|Montage|PlayMontage _skeletalmeshcomponent _animmontage))

(fn ConstructionScript
  (bind _fightersdatatable (Variables|Default|GetFightersDataTable))
  (bind _structurearray (Variables|Default|GetStructureArray))
  (bind _outrownames (DataTable|GetDataTableRowNames _fightersdatatable))
  (for _array_element _outrownames
    (bind _returnvalue (Utilities|GetDataTableRow _fightersdatatable _array_element)
      (:then
        (Utilities|Array|AddUnique _structurearray _returnvalue))))
  (for (_array_element_2 _array_index) _structurearray
    (bind _returnvalue_2 (AddComponent|AddSkeletalMeshComponent false))
    (Components|SkeletalMesh|SetSkeletalMeshAsset _returnvalue_2 (.SkeletalMesh (Utilities|Struct|BreakF_Fighters _array_element_2)))
    (Class|SkeletalMeshComponent|SetAnimClass _returnvalue_2 (Utilities|GetClass (.AnimBlueprint (Utilities|Struct|BreakF_Fighters _array_element_2))))
    (Rendering|SetVisibility _returnvalue_2 false false)
    (Utilities|Array|SetArrayElem _structurearray _array_index (Utilities|Struct|MakeF_Fighters (.SkeletalMesh (Utilities|Struct|BreakF_Fighters _array_element_2)) _returnvalue_2 (.AnimBlueprint (Utilities|Struct|BreakF_Fighters _array_element_2)) (.AnimMontage (Utilities|Struct|BreakF_Fighters _array_element_2))))))