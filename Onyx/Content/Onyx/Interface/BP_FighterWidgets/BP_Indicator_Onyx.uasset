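; BP_Indicator_Onyx is a short-lived floating indicator actor that displays an Onyx value through its OnyxWidget component.
; On BeginPlay it passes Onyx to the widget by interface message and gets direction vectors from player 0's character.
; A timeline lerps it from its spawn point to a randomized offset, upward and against the right vector in that character's frame, then destroys it.
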(event EventBeginPlay
  (Class|BPIIndicator|IFSetOnyx(Message) (UserInterface|GetWidget (Variables|Default|GetOnyxWidget)) (Variables|Default|GetOnyx))
  (bind _output_get (Variables|Default|SetStartPosition (Transformation|GetActorLocation)))
  (bind (_up_vector _right_vector) (Class|BPIPlayer|IFGetVectors(Message) (Game|GetPlayerCharacter 0)))
  (Variables|Default|SetEndPosition (+ _output_get (* _up_vector (Math|Random|RandomFloatinRange 1.2e+02 1.6e+02)) (* _right_vector (Math|Random|RandomFloatinRange -2e+01 -1e+02))))
  (bind _newtrack_0 (Timeline|Timeline Play)
    (:Update
      (Transformation|SetActorLocation (Math|Vector|Lerp(Vector) (Variables|Default|GetStartPosition) (Variables|Default|GetEndPosition) _newtrack_0) false false))
    (:Finished
      (Actor|DestroyActor))))

(fn ConstructionScript)