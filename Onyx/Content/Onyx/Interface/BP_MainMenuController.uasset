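; Main menu controller that handles the back/decline input for navigating the menu overlay.
; BeginPlay caches the menu game mode and game instance.
; On decline completed, a play menu on switcher page 4 returns to its last mode and refocuses the select-mode button.
; Otherwise, any active screen other than the main menu pushes WBP_MainMenu onto the game mode's overlay.
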(event Input|EnhancedActionEvents|EnhancedInputActionIA_NavMenu_Decline
  (params (ActionValue :type Boolean) (ElapsedSeconds :type Float%20%28double-precision%29) (TriggeredSeconds :type Float%20%28double-precision%29) (InputAction :type Input%20Action%20Object%20Reference :default "/Game/Onyx/Input/Actions/IA_NavMenu_Decline.IA_NavMenu_Decline"))
  (bind _gamemode (Variables|Default|GetGameMode))
  (bind _widgetoverlay (Variables|/Game/Onyx/Interface/MainMenu/BP_MenuGameMode.BP_MenuGameMode_C|GetWidgetOverlay _gamemode))
  (bind _menuoverlay (Variables|/Game/Onyx/Interface/WBP_ContainerWidget.WBP_ContainerWidget_C|GetMenuOverlay _widgetoverlay))
  (bind _returnvalue (Class|CommonActivatableWidgetContainerBase|GetActiveWidget _menuoverlay))
  (:Completed
    (Utilities|IsValid _returnvalue
      (:Is%20Valid
        (bind _aswbp_play_menu (Utilities|Casting|CastToWBP_PlayMenu _returnvalue)
          (:then
            (Variables|Default|SetPlayMenu _aswbp_play_menu)
            (if (== (Class|WidgetSwitcher|GetActiveWidgetIndex (Variables|/Game/Onyx/Interface/MainMenu/WBP_PlayMenu.WBP_PlayMenu_C|GetSelectModeSiwtcher _aswbp_play_menu)) 4)
              (Class|WidgetSwitcher|SetActiveWidgetIndex (Variables|/Game/Onyx/Interface/MainMenu/WBP_PlayMenu.WBP_PlayMenu_C|GetSelectModeSiwtcher (Variables|Default|GetPlayMenu)) (Variables|/Game/Onyx/Interface/MainMenu/WBP_PlayMenu.WBP_PlayMenu_C|GetLastMode (Variables|Default|GetPlayMenu)))
              (Class|Widget|SetUserFocus (Variables|/Game/Onyx/Interface/UI_Style/WBP_MyButton.WBP_MyButton_C|GetButtonInvisible (Variables|/Game/Onyx/Interface/MainMenu/WBP_PlayMenu.WBP_PlayMenu_C|GetWBP_MyButton_SelectMode (Variables|Default|GetPlayMenu))) (Class|GameplayStatics|GetPlayerControllerfromID))
              (else
                (Default|PushMenuOverlay (Variables|/Game/Onyx/Interface/MainMenu/BP_MenuGameMode.BP_MenuGameMode_C|GetWidgetOverlay (Variables|Default|GetGameMode)) "/Game/Onyx/Interface/MainMenu/WBP_MainMenu.WBP_MainMenu_C" :!label _label))))
          (:CastFailed
            (Utilities|Casting|CastToWBP_MainMenu _returnvalue
              (:CastFailed
                (goto _label)))))))))

(event EventBeginPlay
  (bind _asbp_menu_game_mode (Utilities|Casting|CastToBP_MenuGameMode (Game|GetGameMode)))
  (Variables|Default|SetGameMode _asbp_menu_game_mode)
  (bind _asbp_game_instance (Utilities|Casting|CastToBP_GameInstance (Game|GetGameInstance)))
  (Variables|Default|SetGameInstance _asbp_game_instance))

(event EventTick
  (params (DeltaSeconds :type Float%20%28single-precision%29)))

(fn ConstructionScript)