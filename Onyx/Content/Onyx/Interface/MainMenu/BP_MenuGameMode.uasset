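; Main menu game mode that sets up the menu scene and UI when play begins.
; BeginPlay points the first player's view at the level's CameraActor, then creates the WBP_ContainerWidget overlay and pushes WBP_MainMenu onto it.
; ShowFighter unhides a randomly chosen SkeletalMeshActor as the displayed fighter, assuming the level holds at least five.
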(event Custom|AddWidgetOverlay
  (bind _returnvalue (UserInterface|CreateWidget "/Game/Onyx/Interface/WBP_ContainerWidget.WBP_ContainerWidget_C"))
  (Variables|Default|SetWidgetOverlay _returnvalue)
  (UserInterface|Viewport|AddtoViewport _returnvalue 0)
  (Default|PushMenuOverlay _returnvalue "/Game/Onyx/Interface/MainMenu/WBP_MainMenu.WBP_MainMenu_C"))

(event Custom|ShowFighter
  (bind _outactors (Actor|GetAllActorsOfClass "/Script/Engine.SkeletalMeshActor"))
  (Rendering|SetActorHiddenInGame (Utilities|Array|Get(acopy) _outactors (Math|Random|RandomInteger 5)) false))

(event EventBeginPlay
  (bind _returnvalue (Actor|GetActorOfClass "/Script/Engine.CameraActor"))
  (Game|Player|SetViewTargetwithBlend (Game|GetPlayerController 0) _returnvalue 0.0 "VTBlend_Linear" 0.0 false)
  (CallFunction|AddWidgetOverlay)
  (CallFunction|ShowFighter))

(fn ConstructionScript)