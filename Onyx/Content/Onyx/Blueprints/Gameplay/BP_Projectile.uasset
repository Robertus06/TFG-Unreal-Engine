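; BP_Projectile is a gameplay projectile that applies a damage Gameplay Effect to fighters on opposing teams.
; Its lifespan derives from Range divided by initial speed.
; On sphere overlap it skips the instigator and uses CompareTeamTag to filter by team tag or ability-system interface.
; Qualifying fighters with an ability system component receive the stored damage spec, and the projectile destroys itself on any qualifying overlap.
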(event OnComponentBeginOverlap(Sphere)
  (params (OverlappedComponent :type Primitive%20Component%20Object%20Reference) (OtherActor :type Actor%20Object%20Reference) (OtherComp :type Primitive%20Component%20Object%20Reference) (OtherBodyIndex :type Integer) (bFromSweep :type Boolean) (SweepResult :type Hit%20Result%20Structure%20%28by%20ref%29))
  (bind _returnvalue (Game|GetInstigator))
  (if (!= OtherActor _returnvalue)
    (Utilities|CompareTeamTag _returnvalue OtherActor
      (:else
        (bind _asbp_fighter (Utilities|Casting|CastToBP_Fighter OtherActor)
          (:then
            (if (Utilities|IsValid (Ability|GetAbilitySystemComponent _asbp_fighter))
              (GameplayEffects|ApplyGameplayEffectSpecToSelf (Ability|GetAbilitySystemComponent _asbp_fighter) (Variables|Default|GetDamageEffectSpecHandle))
              (Actor|DestroyActor)
              (else
                (Actor|DestroyActor :!label _label))))
          (:CastFailed
            (goto _label)))))))

(event EventBeginPlay
  (Actor|SetLifeSpan (/ (Variables|Default|GetRange) (Variables|/Script/Engine.ProjectileMovementComponent|GetInitialSpeed (Variables|Default|GetProjectileMovement)))))

(fn ConstructionScript)