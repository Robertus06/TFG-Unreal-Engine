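; Game mode for an Onyx fighting match, named as the AI variant, that runs the round from spawn to results.
; Spawns local players as their selected fighters at tagged PlayerStarts, applying skins and team colours, then runs a countdown with input disabled for player 0.
; The first death, or lowest health ratio when the timer expires, ends the round and opens GameResults.
; Health, mana, shield and ability changes are forwarded to the active HUD widget.
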(event Custom|Starter%20Countdown
  (bind _returnvalue (UserInterface|CreateWidget "/Game/Onyx/Interface/FightCountdown/WBP_Countdown.WBP_Countdown_C"))
  (Variables|Default|SetCountdownMenu _returnvalue)
  (UserInterface|Viewport|AddtoViewport _returnvalue 0)
  (bind _returnvalue_2 (Utilities|Time|SetTimerbyEvent (delegate Custom|CustomEvent) 1.0 true))
  (Input|DisableInput (Game|GetPlayerController 0))
  (Audio|PlaySound2D "/Game/Onyx/FxSounds/PM_TS_Camera_Film_35mm_SLR_PRACTIKA_DTL3_MKH8040_28_Shutter_Release_1_60th_28.PM_TS_Camera_Film_35mm_SLR_PRACTIKA_DTL3_MKH8040_28_Shutter_Release_1_60th_28" 1.0 1.0 0.0 0 0))

(event Custom|CustomEvent
  (Math|Integer|DecrementInt (Variables|Default|GetCount)
    (:%20%20
      (Rendering|Components|TextRender|SetText (Variables|/Game/Onyx/Interface/FightCountdown/WBP_Countdown.WBP_Countdown_C|GetCountdown (Variables|Default|GetCountdownMenu)) (Utilities|Text|ToText(Integer) (Variables|Default|GetCount)))
      (if (> (Variables|Default|GetCount) 0)
        (Audio|PlaySound2D "/Game/Onyx/FxSounds/PM_TS_Camera_Film_35mm_SLR_PRACTIKA_DTL3_MKH8040_28_Shutter_Release_1_60th_28.PM_TS_Camera_Film_35mm_SLR_PRACTIKA_DTL3_MKH8040_28_Shutter_Release_1_60th_28" 1.0 1.0 0.0 0 0)
        (elif (== (Variables|Default|GetCount) 0)
          (Rendering|Components|TextRender|SetText (Variables|/Game/Onyx/Interface/FightCountdown/WBP_Countdown.WBP_Countdown_C|GetCountdown (Variables|Default|GetCountdownMenu)) "FIGHT")
          (Audio|PlaySound2D "/Game/Onyx/FxSounds/technology_camera_shutter_release_nikon_f4_002.technology_camera_shutter_release_nikon_f4_002" 1.0 1.0 0.0 0 0)
          (elif (< (Variables|Default|GetCount) 0)
            (Utilities|Time|ClearandInvalidateTimerbyHandle (stale Custom|Starter%20Countdown _returnvalue_2))
            (Widget|RemovefromParent (Variables|Default|GetCountdownMenu))
            (Input|EnableInput (Game|GetPlayerController 0))
            (bind _returnvalue (Utilities|Time|SetTimerbyEvent (delegate Custom|EndTime) 3e+02))))))))

(event Custom|Starter%20UI
  (bind _returnvalue (UserInterface|CreateWidget "/Game/Onyx/Interface/WBP_ContainerWidget.WBP_ContainerWidget_C"))
  (Variables|Default|SetUserInterface _returnvalue)
  (UserInterface|Viewport|AddtoViewport _returnvalue 0)
  (Default|PushMenuOverlay (Variables|Default|GetUserInterface) "/Game/Onyx/Interface/InGame_Interface/WBP_InGame_Interface_AI.WBP_InGame_Interface_AI_C"))

(event Custom|EndTime
  (Utilities|Time|ClearandInvalidateTimerbyHandle (stale Custom|CustomEvent _returnvalue))
  (for _index (range 0 (- (Variables|/Game/Onyx/GameCore/BP_GameInstance.BP_GameInstance_C|GetNumPlayers (Variables|Default|GetGameInstance)) 1))
    (Utilities|Array|Add (Variables|Default|GetAuxHealPlayers) (/ (.ReturnValue (Class|AbilitySystemComponent|GetGameplayAttributeValue (Ability|GetAbilitySystemComponent (Game|GetPlayerCharacter _index)) "(AttributeName=\"Health\",Attribute=/Script/Onyx.OnyxAttributeSet:Health,AttributeOwner=\"/Script/CoreUObject.Class'/Script/Onyx.OnyxAttributeSet'\")")) (.ReturnValue (Class|AbilitySystemComponent|GetGameplayAttributeValue (Ability|GetAbilitySystemComponent (Game|GetPlayerCharacter _index)) "(AttributeName=\"MaxHealth\",Attribute=/Script/Onyx.OnyxAttributeSet:MaxHealth,AttributeOwner=\"/Script/CoreUObject.Class'/Script/Onyx.OnyxAttributeSet'\")")))))
  (Utilities|Array|AddUnique (Variables|Default|GetDeadPlayers) (.IndexOfMinValue (Math|Float|MinOfFloatArray (Variables|Default|GetAuxHealPlayers))))
  (CallFunction|EndRound))

(event Custom|ChangeHealth
  (params (PlayerID :type Integer) (PercentValue :type Float%20%28double-precision%29))
  (bind _userinterface (Variables|Default|GetUserInterface))
  (Utilities|IsValid _userinterface
    (:Is%20Valid
      (Class|BPIinGameUI|ChangeHealth(Message) (Class|CommonActivatableWidgetContainerBase|GetActiveWidget (Variables|/Game/Onyx/Interface/WBP_ContainerWidget.WBP_ContainerWidget_C|GetMenuOverlay _userinterface)) PlayerID PercentValue))))

(event Custom|ChangeMana
  (params (PlayerID :type Integer) (Percent%20Value :type Float%20%28double-precision%29))
  (bind _userinterface (Variables|Default|GetUserInterface))
  (Utilities|IsValid _userinterface
    (:Is%20Valid
      (Class|BPIinGameUI|ChangeMana(Message) (Class|CommonActivatableWidgetContainerBase|GetActiveWidget (Variables|/Game/Onyx/Interface/WBP_ContainerWidget.WBP_ContainerWidget_C|GetMenuOverlay _userinterface)) PlayerID Percent%20Value))))

(event Custom|ChangeShield
  (params (PlayerID :type Integer) (Percent%20Value :type Float%20%28double-precision%29))
  (bind _userinterface (Variables|Default|GetUserInterface))
  (Utilities|IsValid _userinterface
    (:Is%20Valid
      (Class|BPIinGameUI|ChangeShield(Message) (Class|CommonActivatableWidgetContainerBase|GetActiveWidget (Variables|/Game/Onyx/Interface/WBP_ContainerWidget.WBP_ContainerWidget_C|GetMenuOverlay _userinterface)) PlayerID Percent%20Value))))

(event Custom|EndRound
  (Utilities|Array|AddUnique (Variables|/Game/Onyx/GameCore/BP_GameInstance.BP_GameInstance_C|GetPlayersPosition (Variables|Default|GetGame%20Instance)) (Utilities|Array|Get(acopy) (Variables|Default|GetDeadPlayers)))
  (Game|OpenLevel(byObjectReference) "/Game/Onyx/Levels/GameResults.GameResults"))

(event Custom|ChangeAbility
  (params (AbilityIndex :type Integer) (Character :type Integer) (Cooldown :type Float%20%28double-precision%29))
  (bind _userinterface (Variables|Default|GetUserInterface))
  (Utilities|IsValid _userinterface
    (:Is%20Valid
      (Class|BPIinGameUI|ChangeAbility(Message) (Class|CommonActivatableWidgetContainerBase|GetActiveWidget (Variables|/Game/Onyx/Interface/WBP_ContainerWidget.WBP_ContainerWidget_C|GetMenuOverlay _userinterface)) AbilityIndex Character Cooldown))))

(event EventBeginPlay
  (CallFunction|StarterUI)
  (CallFunction|SpawnPlayers)
  (bind _returnvalue (Actor|GetActorOfClass "/Game/Onyx/GameCore/BP_MainCamera.BP_MainCamera_C"))
  (Class|MainCamera|InitializeCamera _returnvalue)
  (CallFunction|StarterCountdown)
  (bind _returnvalue_2 (UserInterface|CreateWidget "/Game/Onyx/Interface/WBP_ContainerWidget.WBP_ContainerWidget_C"))
  (Variables|Default|SetCrateOverlay _returnvalue_2)
  (UserInterface|Viewport|AddtoViewport _returnvalue_2 0)
  (bind _returnvalue_3 (UserInterface|CreateWidget "/Game/Onyx/Interface/WBP_ContainerWidget.WBP_ContainerWidget_C"))
  (Variables|Default|SetOverlay _returnvalue_3)
  (UserInterface|Viewport|AddtoViewport _returnvalue_3 0))

(event EventPlayerDead
  (params (PlayerID :type Integer))
  (Utilities|Array|AddUnique (Variables|Default|GetDeadPlayers) PlayerID)
  (CallFunction|EndRound))

(fn ConstructionScript
  (bind _asbp_game_instance (Utilities|Casting|CastToBP_GameInstance (Game|GetGameInstance)))
  (bind _output_get (Variables|Default|SetGame%20Instance _asbp_game_instance))
  (CallFunction|DefaultClass (.fighterselected (Utilities|Array|Get(acopy) (Variables|/Game/Onyx/GameCore/BP_GameInstance.BP_GameInstance_C|GetPlayerSelection _output_get)))))

(fn SpawnPlayers
  (Utilities|FlowControl|Sequence
    (:then_0
      (bind _asbp_game_instance (Utilities|Casting|CastToBP_GameInstance (Game|GetGameInstance)))
      (Variables|Default|SetGameInstance _asbp_game_instance))
    (:then_1
      (for _index (range 0 (- (Variables|/Game/Onyx/GameCore/BP_GameInstance.BP_GameInstance_C|GetNumPlayers (Variables|Default|GetGameInstance)) 1))
        (Utilities|IsValid (Class|GameplayStatics|GetPlayerControllerfromID _index)
          (:Is%20Valid
            (Class|GameplayStatics|RemovePlayer (Class|GameplayStatics|GetPlayerControllerfromID _index) true))
          (:Is%20Not%20Valid
            _))
        (CallFunction|DefaultClass (.fighterselected (Utilities|Array|Get(acopy) (Variables|/Game/Onyx/GameCore/BP_GameInstance.BP_GameInstance_C|GetPlayerSelection (Variables|Default|GetGame%20Instance)) _index)))
        (bind _returnvalue (Class|GameplayStatics|CreatePlayer _index))
        (Input|AddMappingContext (PlayerController|LocalPlayerSubsystems|GetEnhancedInputLocalPlayerSubsystem _returnvalue) "/Game/Onyx/Input/IMC_Default.IMC_Default" 0 "(bIgnoreAllPressedKeysUntilRelease=True,bForceImmediately=False,bNotifyUserSettings=False)"))
      (bind _outactors (Actor|GetAllActorsOfClass "/Script/Engine.PlayerStart"))
      (for _array_element _outactors
        (bind _asbp_fighter (Utilities|Casting|CastToBP_Fighter (Game|GetPlayerCharacter (Math|Conversions|ToInteger(Byte) (Utilities|String|ToString(Name) (Variables|/Script/Engine.PlayerStart|GetPlayerStartTag _array_element))))))
        (bind _output_get (Variables|Default|SetFighter _asbp_fighter))
        (Variables|/Game/Onyx/Character/BP_Fighter.BP_Fighter_C|SetTarget%20Rotation _asbp_fighter (Transformation|GetActorRotation _array_element))
        (Variables|/Script/Onyx.OnyxCharacter|SetCharacterID _output_get (Math|Conversions|ToInteger(Byte) (Utilities|String|ToString(Name) (Variables|/Script/Engine.PlayerStart|GetPlayerStartTag _array_element))))
        (bind _returnvalue_2 (Utilities|GetDataTableRow "/Game/Onyx/Interface/SelectFighter/DT_Skins.DT_Skins" (.fighterselected (Utilities|Array|Get(acopy) (Variables|/Game/Onyx/GameCore/BP_GameInstance.BP_GameInstance_C|GetPlayerSelection (Variables|Default|GetGame%20Instance)) (Math|Conversions|ToInteger(Byte) (Utilities|String|ToString(Name) (Variables|/Script/Engine.PlayerStart|GetPlayerStartTag _array_element))))))
          (:then
            (Default|SetSkin (Variables|Default|GetFighter) (Utilities|Array|Get(acopy) (Utilities|Struct|BreakF_Skins _returnvalue_2) (.skinselected (Utilities|Array|Get(acopy) (Variables|/Game/Onyx/GameCore/BP_GameInstance.BP_GameInstance_C|GetPlayerSelection (Variables|Default|GetGame%20Instance)) (Math|Conversions|ToInteger(Byte) (Utilities|String|ToString(Name) (Variables|/Script/Engine.PlayerStart|GetPlayerStartTag _array_element)))))))
            (Transformation|SetActorTransform (Game|GetPlayerCharacter (Math|Conversions|ToInteger(Byte) (Utilities|String|ToString(Name) (Variables|/Script/Engine.PlayerStart|GetPlayerStartTag _array_element)))) (Transformation|GetActorTransform _array_element))
            (CallFunction|ChangeTeamColor (Math|Conversions|ToInteger(Byte) (Utilities|String|ToString(Name) (Variables|/Script/Engine.PlayerStart|GetPlayerStartTag _array_element))))))))))

(fn DefaultClass
  (params (Selection :type Name))
  (switch name Selection
    (:Countess
      (Variables|Default|SetDefaultPawnClass "/Game/Onyx/Character/Countess/BP_Countess.BP_Countess_C"))
    (:Grim
      (Variables|Default|SetDefaultPawnClass "/Game/Onyx/Character/Grim/BP_Grim.BP_Grim_C"))
    (:Grux
      (Variables|Default|SetDefaultPawnClass "/Game/Onyx/Character/Grux/BP_Grux.BP_Grux_C"))
    (:Iggy
      (Variables|Default|SetDefaultPawnClass "/Game/Onyx/Character/Iggy/BP_Iggy.BP_Iggy_C"))
    (:Khaimera
      (Variables|Default|SetDefaultPawnClass "/Game/Onyx/Character/Khaimera/BP_Khaimera.BP_Khaimera_C"))
    (:Phase
      (Variables|Default|SetDefaultPawnClass "/Game/Onyx/Character/Phase/BP_Phase.BP_Phase_C"))
    (:Sevarog
      (Variables|Default|SetDefaultPawnClass "/Game/Onyx/Character/Sevarog/BP_Sevarog.BP_Sevarog_C"))
    (:Sparrow
      (Variables|Default|SetDefaultPawnClass "/Game/Onyx/Character/Sparrow/BP_Sparrow.BP_Sparrow_C"))
    (:Terra
      (Variables|Default|SetDefaultPawnClass "/Game/Onyx/Character/Terra/BP_Terra.BP_Terra_C"))))

(fn ChangeTeamColor
  (params (Index :type Integer))
  (bind _game_instance (Variables|Default|GetGame%20Instance))
  (bind _fighter (Variables|Default|GetFighter))
  (bind _fighter_2 (Variables|Default|GetFighter))
  (bind _fighter_3 (Variables|Default|GetFighter))
  (if (and (== (Variables|/Game/Onyx/GameCore/BP_GameInstance.BP_GameInstance_C|GetNumTeams _game_instance) 2) (== (Variables|/Game/Onyx/GameCore/BP_GameInstance.BP_GameInstance_C|GetNumPlayers _game_instance) 4))
    (if (or (== Index 2) (== Index 0))
      (Class|WidgetComponent|SetTintColorandOpacity (Variables|/Game/Onyx/Character/BP_Fighter.BP_Fighter_C|GetIndicator_Arrow _fighter) (Utilities|Array|Get(acopy) (Variables|/Game/Onyx/GameCore/BP_GameInstance.BP_GameInstance_C|GetTeamColors (Variables|Default|GetGame%20Instance))))
      (Variables|/Script/Onyx.OnyxCharacter|SetTeamTag _fighter "(TagName=\"Team.Green\")")
      (else
        (Class|WidgetComponent|SetTintColorandOpacity (Variables|/Game/Onyx/Character/BP_Fighter.BP_Fighter_C|GetIndicator_Arrow _fighter_3) (Utilities|Array|Get(acopy) (Variables|/Game/Onyx/GameCore/BP_GameInstance.BP_GameInstance_C|GetTeamColors (Variables|Default|GetGame%20Instance)) 1))
        (Variables|/Script/Onyx.OnyxCharacter|SetTeamTag _fighter_3 "(TagName=\"Team.Red\")")))
    (else
      (Class|WidgetComponent|SetTintColorandOpacity (Variables|/Game/Onyx/Character/BP_Fighter.BP_Fighter_C|GetIndicator_Circle _fighter_2) (Utilities|Array|Get(acopy) (Variables|/Game/Onyx/GameCore/BP_GameInstance.BP_GameInstance_C|GetTeamColors (Variables|Default|GetGame%20Instance)) Index))
      (switch int Index
        (:0
          (Variables|/Script/Onyx.OnyxCharacter|SetTeamTag _fighter_2 "(TagName=\"Team.Green\")"))
        (:1
          (Variables|/Script/Onyx.OnyxCharacter|SetTeamTag _fighter_2 "(TagName=\"Team.Red\")"))
        (:2
          (Variables|/Script/Onyx.OnyxCharacter|SetTeamTag _fighter_2 "(TagName=\"Team.Blue\")"))
        (:3
          (Variables|/Script/Onyx.OnyxCharacter|SetTeamTag _fighter_2 "(TagName=\"Team.Yellow\")"))))))