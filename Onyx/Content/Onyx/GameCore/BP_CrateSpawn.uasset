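; Crate spawner actor that keeps a single BP_Crate in the level and announces each new one on screen.
; After a short startup delay, a looping timer checks for existing crates and, if none remain, spawns one at a random TargetPoint's transform.
; It then pushes a WBP_CrateSpawn notice onto the game mode's crate overlay, if no widget is active, and removes it after a few seconds.
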(event Custom|CustomEvent
  (bind _as_bp_onyx_game_mode (Variables|Default|GetAs%20BP%20Onyx%20Game%20Mode))
  (bind _crateoverlay (Variables|/Game/Onyx/GameCore/BP_OnyxGameMode.BP_OnyxGameMode_C|GetCrateOverlay _as_bp_onyx_game_mode))
  (bind _outactors (Actor|GetAllActorsOfClass "/Game/Onyx/Character/Crate/BP_Crate.BP_Crate_C"))
  (if (not (> (Utilities|Array|Length _outactors) 0))
    (CallFunction|Spawner)
    (Utilities|IsValid (Class|CommonActivatableWidgetContainerBase|GetActiveWidget (Variables|/Game/Onyx/Interface/WBP_ContainerWidget.WBP_ContainerWidget_C|GetMenuOverlay _crateoverlay))
      (:Is%20Not%20Valid
        (Default|PushMenuOverlay _crateoverlay "/Game/Onyx/Interface/InGame_Interface/WBP_CrateSpawn.WBP_CrateSpawn_C")
        (bind _returnvalue (Utilities|Time|SetTimerbyEvent (delegate Custom|CustomEvent_0) 5.0))))))

(event Custom|CustomEvent_0
  (bind _as_bp_onyx_game_mode (Variables|Default|GetAs%20BP%20Onyx%20Game%20Mode))
  (bind _crateoverlay (Variables|/Game/Onyx/GameCore/BP_OnyxGameMode.BP_OnyxGameMode_C|GetCrateOverlay _as_bp_onyx_game_mode))
  (bind _menuoverlay (Variables|/Game/Onyx/Interface/WBP_ContainerWidget.WBP_ContainerWidget_C|GetMenuOverlay _crateoverlay))
  (bind _returnvalue (Class|CommonActivatableWidgetContainerBase|GetActiveWidget _menuoverlay))
  (Utilities|Time|ClearandInvalidateTimerbyHandle (stale Custom|CustomEvent _returnvalue))
  (Utilities|IsValid _returnvalue
    (:Is%20Valid
      (Default|RemoveMenuOverlay _crateoverlay _returnvalue))))

(event Custom|CustomEvent_1
  (Utilities|Time|ClearandInvalidateTimerbyHandle (stale EventBeginPlay _returnvalue))
  (Utilities|Time|SetTimerbyEvent (delegate Custom|CustomEvent) 3e+01 true))

(event EventBeginPlay
  (bind _asbp_onyx_game_mode (Utilities|Casting|CastToBP_OnyxGameMode (Game|GetGameMode)))
  (Variables|Default|SetAs%20BP%20Onyx%20Game%20Mode _asbp_onyx_game_mode)
  (bind _returnvalue (Utilities|Time|SetTimerbyEvent (delegate Custom|CustomEvent_1) 4.0)))

(event Collision|EventActorBeginOverlap
  (params (OtherActor :type Actor%20Object%20Reference)))

(event EventTick
  (params (DeltaSeconds :type Float%20%28single-precision%29)))

(fn ConstructionScript)

(fn Spawner
  (bind _outactors (Actor|GetAllActorsOfClass "/Script/Engine.TargetPoint"))
  (bind _output_get (Variables|Default|SetSpawn%20Positions _outactors))
  (Game|SpawnActorfromClass "/Game/Onyx/Character/Crate/BP_Crate.BP_Crate_C" (Transformation|GetActorTransform (.OutItem (Utilities|Array|Random _output_get))) "Undefined" "MultiplyWithRoot" 0 0))