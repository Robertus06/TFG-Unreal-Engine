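; Game mode for local multiplayer fighter rounds, configured from BP_GameInstance's player selections and team settings.
; It switches DefaultPawnClass before creating each local player, then applies skins, PlayerStart transforms by tag, and team-colored indicators.
; It shows a matching HUD and a countdown that locks only player 0's input, then runs a round timer.
; At round end, placeholder logic damages a random team index's health, scaled by round, then opens the shop level.
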(event Custom|Starter%20Countdown
  (bind _returnvalue (UserInterface|CreateWidget "/Game/Onyx/Interface/FightCountdown/WBP_Countdown.WBP_Countdown_C"))
  (Variables|Default|SetCountdownMenu _returnvalue)
  (UserInterface|Viewport|AddtoViewport _returnvalue 0)
  (bind _returnvalue_2 (Utilities|Time|SetTimerbyEvent (delegate Custom|CustomEvent) 1.0 true))
  (Input|DisableInput (Game|GetPlayerCharacter 0) (Game|GetPlayerController 0)))

(event Custom|CustomEvent
  (Math|Integer|DecrementInt (Variables|Default|GetCount)
    (:%20%20
      (Rendering|Components|TextRender|SetText (Variables|/Game/Onyx/Interface/FightCountdown/WBP_Countdown.WBP_Countdown_C|GetCountdown (Variables|Default|GetCountdownMenu)) (Utilities|Text|ToText(Integer) (Variables|Default|GetCount)))
      (if (< (Variables|Default|GetCount) 1)
        (Rendering|Components|TextRender|SetText (Variables|/Game/Onyx/Interface/FightCountdown/WBP_Countdown.WBP_Countdown_C|GetCountdown (Variables|Default|GetCountdownMenu)) "FIGHT")
        (if (< (Variables|Default|GetCount) 0)
          (Utilities|Time|ClearandInvalidateTimerbyHandle (stale Custom|Starter%20Countdown _returnvalue_2))
          (Widget|RemovefromParent (Variables|Default|GetCountdownMenu))
          (Input|EnableInput (Game|GetPlayerCharacter 0) (Game|GetPlayerController 0))
          (bind _returnvalue (Utilities|Time|SetTimerbyEvent (delegate Custom|EndRound) 1.0 true)))))))

(event Custom|Starter%20UI
  (bind _returnvalue (UserInterface|CreateWidget "/Game/Onyx/Interface/WBP_ContainerWidget.WBP_ContainerWidget_C"))
  (Variables|Default|SetUserInterface _returnvalue)
  (UserInterface|Viewport|AddtoViewport _returnvalue 0)
  (if (== (Variables|/Game/Onyx/GameCore/BP_GameInstance.BP_GameInstance_C|GetNumPlayers (Variables|Default|GetGame%20Instance)) 2)
    (Default|PushMenuOverlay (Variables|Default|GetUserInterface) "/Game/Onyx/Interface/InGame_Interface/WBP_InGame_Interface_2_Players.WBP_InGame_Interface_2_Players_C")
    (elif (== (Variables|/Game/Onyx/GameCore/BP_GameInstance.BP_GameInstance_C|GetNumTeams (Variables|Default|GetGame%20Instance)) 2)
      (Default|PushMenuOverlay (Variables|Default|GetUserInterface) "/Game/Onyx/Interface/InGame_Interface/WBP_InGame_Interface_2_Teams.WBP_InGame_Interface_2_Teams_C")
      (else
        (Default|PushMenuOverlay (Variables|Default|GetUserInterface) "/Game/Onyx/Interface/InGame_Interface/WBP_InGame_Interface_4_Players.WBP_InGame_Interface_4_Players_C")))))

(event Custom|EndRound
  (Math|Integer|DecrementInt (Variables|Default|GetRoundCount)
    (:%20%20
      (if (< (Variables|Default|GetRoundCount) 0)
        (Utilities|Time|ClearandInvalidateTimerbyHandle (stale Custom|CustomEvent _returnvalue))
        (CallFunction|SubtractHealthLoser (Math|Random|RandomIntegerinRange 0 (- (Variables|/Game/Onyx/GameCore/BP_GameInstance.BP_GameInstance_C|GetNumTeams (Variables|Default|GetGame%20Instance)) 1)))
        (Game|OpenLevel(byObjectReference) "/Game/Onyx/Levels/ShopMenu.ShopMenu")))))

(event EventBeginPlay
  (CallFunction|SpawnPlayers)
  (CallFunction|StarterUI)
  (CallFunction|StarterCountdown)
  (bind _returnvalue (UserInterface|CreateWidget "/Game/Onyx/Interface/WBP_ContainerWidget.WBP_ContainerWidget_C"))
  (Variables|Default|SetOverlay _returnvalue)
  (UserInterface|Viewport|AddtoViewport _returnvalue 0))

(fn ConstructionScript
  (bind _asbp_game_instance (Utilities|Casting|CastToBP_GameInstance (Game|GetGameInstance)))
  (bind _output_get (Variables|Default|SetGame%20Instance _asbp_game_instance))
  (CallFunction|DefaultClass (.fighterselected (Utilities|Array|Get(acopy) (Variables|/Game/Onyx/GameCore/BP_GameInstance.BP_GameInstance_C|GetPlayerSelection _output_get)))))

(fn SpawnPlayers
  (Utilities|FlowControl|Sequence
    (:then_0
      (bind _asbp_game_instance (Utilities|Casting|CastToBP_GameInstance (Game|GetGameInstance)))
      (Variables|Default|SetGameInstance _asbp_game_instance))
    (:then_1
      (for _index (range 1 (- (Variables|/Game/Onyx/GameCore/BP_GameInstance.BP_GameInstance_C|GetNumPlayers (Variables|Default|GetGameInstance)) 1))
        (CallFunction|DefaultClass (.fighterselected (Utilities|Array|Get(acopy) (Variables|/Game/Onyx/GameCore/BP_GameInstance.BP_GameInstance_C|GetPlayerSelection (Variables|Default|GetGame%20Instance)) _index)))
        (bind _returnvalue (Class|GameplayStatics|CreatePlayer _index))
        (Input|AddMappingContext (PlayerController|LocalPlayerSubsystems|GetEnhancedInputLocalPlayerSubsystem _returnvalue) "/Game/ThirdPerson/Input/IMC_Default.IMC_Default" 0 "(bIgnoreAllPressedKeysUntilRelease=True,bForceImmediately=False,bNotifyUserSettings=False)"))
      (bind _outactors (Actor|GetAllActorsOfClass "/Script/Engine.PlayerStart"))
      (for _array_element _outactors
        (bind _asbp_fighter (Utilities|Casting|CastToBP_Fighter (Game|GetPlayerCharacter (Math|Conversions|ToInteger(Byte) (Utilities|String|ToString(Name) (Variables|/Script/Engine.PlayerStart|GetPlayerStartTag _array_element))))))
        (Variables|Default|SetFighter _asbp_fighter)
        (bind _returnvalue_2 (Utilities|GetDataTableRow "/Game/Onyx/Interface/SelectFighter/DT_Skins.DT_Skins" (.fighterselected (Utilities|Array|Get(acopy) (Variables|/Game/Onyx/GameCore/BP_GameInstance.BP_GameInstance_C|GetPlayerSelection (Variables|Default|GetGame%20Instance)) (Math|Conversions|ToInteger(Byte) (Utilities|String|ToString(Name) (Variables|/Script/Engine.PlayerStart|GetPlayerStartTag _array_element))))))
          (:then
            (Default|SetSkin (Variables|Default|GetFighter) (Utilities|Array|Get(acopy) (Utilities|Struct|BreakF_Skins _returnvalue_2) (.skinselected (Utilities|Array|Get(acopy) (Variables|/Game/Onyx/GameCore/BP_GameInstance.BP_GameInstance_C|GetPlayerSelection (Variables|Default|GetGame%20Instance)) (Math|Conversions|ToInteger(Byte) (Utilities|String|ToString(Name) (Variables|/Script/Engine.PlayerStart|GetPlayerStartTag _array_element)))))))
            (Transformation|SetActorTransform (Game|GetPlayerCharacter (Math|Conversions|ToInteger(Byte) (Utilities|String|ToString(Name) (Variables|/Script/Engine.PlayerStart|GetPlayerStartTag _array_element)))) (Transformation|GetActorTransform _array_element))
            (CallFunction|ChangeTeamColor (Math|Conversions|ToInteger(Byte) (Utilities|String|ToString(Name) (Variables|/Script/Engine.PlayerStart|GetPlayerStartTag _array_element))))))))))

(fn DefaultClass
  (params (Selection :type Name))
  (switch name Selection
    (:Countess
      (Variables|Default|SetDefaultPawnClass "/Game/Onyx/Character/Countess/BP_Countess.BP_Countess_C"))
    (:Grim
      (Variables|Default|SetDefaultPawnClass "/Game/Onyx/Character/Grim/BP_Grim.BP_Grim_C"))
    (:Grux
      (Variables|Default|SetDefaultPawnClass "/Game/Onyx/Character/Grux/BP_Grux.BP_Grux_C"))
    (:Iggy
      (Variables|Default|SetDefaultPawnClass "/Game/Onyx/Character/Iggy/BP_Iggy.BP_Iggy_C"))
    (:Khaimera
      (Variables|Default|SetDefaultPawnClass "/Game/Onyx/Character/Khaimera/BP_Khaimera.BP_Khaimera_C"))
    (:Phase
      (Variables|Default|SetDefaultPawnClass "/Game/Onyx/Character/Phase/BP_Phase.BP_Phase_C"))
    (:Sevarog
      (Variables|Default|SetDefaultPawnClass "/Game/Onyx/Character/Sevarog/BP_Sevarog.BP_Sevarog_C"))
    (:Sparrow
      (Variables|Default|SetDefaultPawnClass "/Game/Onyx/Character/Sparrow/BP_Sparrow.BP_Sparrow_C"))
    (:Terra
      (Variables|Default|SetDefaultPawnClass "/Game/Onyx/Character/Terra/BP_Terra.BP_Terra_C"))))

(fn ChangeTeamColor
  (params (Index :type Integer))
  (bind _game_instance (Variables|Default|GetGame%20Instance))
  (if (and (== (Variables|/Game/Onyx/GameCore/BP_GameInstance.BP_GameInstance_C|GetNumTeams _game_instance) 2) (== (Variables|/Game/Onyx/GameCore/BP_GameInstance.BP_GameInstance_C|GetNumPlayers _game_instance) 4))
    (if (or (== Index 2) (== Index 0))
      (Class|WidgetComponent|SetTintColorandOpacity (Variables|/Game/Onyx/Character/BP_Fighter.BP_Fighter_C|GetIndicator_Arrow (Variables|Default|GetFighter)) (Utilities|Array|Get(acopy) (Variables|/Game/Onyx/GameCore/BP_GameInstance.BP_GameInstance_C|GetTeamColors (Variables|Default|GetGame%20Instance))))
      (else
        (Class|WidgetComponent|SetTintColorandOpacity (Variables|/Game/Onyx/Character/BP_Fighter.BP_Fighter_C|GetIndicator_Arrow (Variables|Default|GetFighter)) (Utilities|Array|Get(acopy) (Variables|/Game/Onyx/GameCore/BP_GameInstance.BP_GameInstance_C|GetTeamColors (Variables|Default|GetGame%20Instance)) 1))))
    (else
      (Class|WidgetComponent|SetTintColorandOpacity (Variables|/Game/Onyx/Character/BP_Fighter.BP_Fighter_C|GetIndicator_Circle (Variables|Default|GetFighter)) (Utilities|Array|Get(acopy) (Variables|/Game/Onyx/GameCore/BP_GameInstance.BP_GameInstance_C|GetTeamColors (Variables|Default|GetGame%20Instance)) Index)))))

(fn SubtractHealthLoser
  (params (Player :type Integer))
  (bind _gameinstance (Variables|Default|GetGameInstance))
  (bind _playerhealth (Variables|/Game/Onyx/GameCore/BP_GameInstance.BP_GameInstance_C|GetPlayerHealth _gameinstance))
  (Utilities|FlowControl|Sequence
    (:then_0
      (if (<= (Variables|/Game/Onyx/GameCore/BP_GameInstance.BP_GameInstance_C|GetRound (Variables|Default|GetGame%20Instance)) 3)
        (Variables|Default|SetDamage 1e+01)
        (elif (and (<= (Variables|/Game/Onyx/GameCore/BP_GameInstance.BP_GameInstance_C|GetRound (Variables|Default|GetGame%20Instance)) 5) (> (Variables|/Game/Onyx/GameCore/BP_GameInstance.BP_GameInstance_C|GetRound (Variables|Default|GetGame%20Instance)) 3))
          (Variables|Default|SetDamage 2e+01)
          (elif (> (Variables|/Game/Onyx/GameCore/BP_GameInstance.BP_GameInstance_C|GetRound (Variables|Default|GetGame%20Instance)) 5)
            (Variables|Default|SetDamage 3e+01)))))
    (:then_1
      (Utilities|Array|SetArrayElem _playerhealth Player (- (Utilities|Array|Get(acopy) _playerhealth Player) (Variables|Default|GetDamage))))))