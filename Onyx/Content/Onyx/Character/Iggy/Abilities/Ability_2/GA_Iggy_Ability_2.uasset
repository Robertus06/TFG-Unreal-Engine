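; Iggy's second gameplay ability, which grants a temporary shield to Iggy.
; On a successful commit it reports the ability index and cooldown to BP_Fighter, then applies GE_AddShield to the owner.
; Set-by-caller tags supply a fixed duration and a shield amount built from a base value plus scaled owner attributes.
; A CompareTeamTag helper for team checks is defined but not called by the activation flow.
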(event Ability|EventActivateAbility
  (bind _returnvalue (Ability|GetOwningActorfromActorInfo))
  (bind _returnvalue_2 (Ability|GetAbilitySystemComponent _returnvalue))
  (bind _returnvalue_3 (Ability|CommitAbility))
  (if _returnvalue_3
    (Utilities|AbilityInfo 2)
    (bind _returnvalue_4 (Ability|GameplayEffect|AssignTagSetbyCallerMagnitude (Ability|MakeOutgoingGameplayEffectSpec "/Game/Onyx/Effects/GE_AddShield.GE_AddShield_C") "(TagName=\"Data.Shield\")" (+ (* (.ReturnValue (Class|AbilitySystemComponent|GetGameplayAttributeValue _returnvalue_2 "(AttributeName=\"MagicResistence\",Attribute=/Script/Onyx.OnyxAttributeSet:MagicResistence,AttributeOwner=\"/Script/CoreUObject.Class'/Script/Onyx.OnyxAttributeSet'\")")) 0.5) (* (.ReturnValue (Class|AbilitySystemComponent|GetGameplayAttributeValue _returnvalue_2 "(AttributeName=\"Armor\",Attribute=/Script/Onyx.OnyxAttributeSet:Armor,AttributeOwner=\"/Script/CoreUObject.Class'/Script/Onyx.OnyxAttributeSet'\")")) 0.5) (Variables|Default|GetShield))))
    (bind _returnvalue_5 (Ability|GameplayEffect|AssignTagSetbyCallerMagnitude _returnvalue_4 "(TagName=\"Data.Duration\")" 5.0))
    (Ability|ApplyGameplayEffectSpecToOwner _returnvalue_5)
    (Ability|EndAbility)
    (else
      (Ability|EndAbility))))

(event Ability|EventOnEndAbility
  (params (bWasCancelled :type Boolean)))