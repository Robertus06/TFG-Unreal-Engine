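; Grim character Blueprint that fires projectiles for its attacks and switches its standard-attack decal when buffed.
; When collision is enabled for the standard attack or the third ability, it calls LaunchProjectile.
; BeginPlay caches both decal components, and SetBuffedDecal points the standard-attack decal variable at the buffed or normal one, then hides the DecalBuffedAttack component.
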(event Custom|Set%20Buffed%20Decal
  (params (IsBuffed :type Boolean))
  (Variables|Default|SetDecal_StandardAttack (select IsBuffed (Variables|Default|GetRef%20Buffed%20Attack) (Variables|Default|GetRef%20Standard%20Attack)))
  (Rendering|SetVisibility (Variables|Default|GetDecal_BuffedAttack) false true))

(event EventBeginPlay
  (|CallParentFunction)
  (Variables|Default|SetRef%20Standard%20Attack (Variables|Default|GetDecal_StandardAttack))
  (Variables|Default|SetRef%20Buffed%20Attack (Variables|Default|GetDecal_BuffedAttack)))

(event Collision|EventActorBeginOverlap
  (params (OtherActor :type Actor%20Object%20Reference)))

(event EventTick
  (params (DeltaSeconds :type Float%20%28single-precision%29))
  (|CallParentFunction DeltaSeconds) ; This node is disabled and will not be called.\nDrag off pins to build functionality.
)

(event EventEnableCollisionAbility
  (params (Ability :type EAbilities%20Enum :default "NewEnumerator0"))
  (switch Utilities|FlowControl|Switch|SwitchonEAbilities Ability
    (:NewEnumerator2
      (CallFunction|LaunchProjectile))
    (:NewEnumerator3
      (CallFunction|LaunchProjectile))))

(fn ConstructionScript
  (|CallParentFunction))