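; Gameplay ability for the Grim character's first ability slot, currently only committing, reporting and ending.
; On successful commit, AbilityInfo passes the slot index and cooldown duration to BP_Fighter's ability-change event.
; A disconnected, never-run chain waits for a damage gameplay event, team-checks it via CompareTeamTag, and applies GE_DealDamage with SetByCaller physical damage from an instigator attribute.
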(event Ability|EventActivateAbility
  (bind _returnvalue (Ability|CommitAbility))
  (if _returnvalue
    (Utilities|AbilityInfo 1)
    (Ability|EndAbility)
    (else
      (Ability|EndAbility))))

(event Ability|EventOnEndAbility
  (params (bWasCancelled :type Boolean)))