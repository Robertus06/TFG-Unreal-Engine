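; BP_Phase is the Phase character Blueprint, which handles hit delivery for its abilities through the Gameplay Ability System.
; EnableCollisionAbility launches a projectile for the standard attack and Ability 1, and runs CommitDamage on dedicated collision components for Abilities 2 and 3.
; CommitDamage gathers overlapping ability-system actors other than itself and sends them as target data in an Event.Damage gameplay event to itself.
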(event EventBeginPlay
  (|CallParentFunction) ; This node is disabled and will not be called.\nDrag off pins to build functionality.
)

(event Collision|EventActorBeginOverlap
  (params (OtherActor :type Actor%20Object%20Reference)))

(event EventTick
  (params (DeltaSeconds :type Float%20%28single-precision%29))
  (|CallParentFunction DeltaSeconds) ; This node is disabled and will not be called.\nDrag off pins to build functionality.
)

(event EventEnableCollisionAbility
  (params (Ability :type EAbilities%20Enum :default "NewEnumerator0"))
  (switch Utilities|FlowControl|Switch|SwitchonEAbilities Ability
    (:NewEnumerator0
      (CallFunction|LaunchProjectile))
    (:NewEnumerator1
      (CallFunction|CommitDamage (Variables|Default|GetAB_02_Coll)))
    (:NewEnumerator2
      (CallFunction|CommitDamage (Variables|Default|GetAB_03_Coll)))
    (:NewEnumerator3
      (CallFunction|LaunchProjectile))))

(fn ConstructionScript
  (|CallParentFunction))

(fn CommitDamage
  (params (Collision :type Primitive%20Component%20Object%20Reference))
  (bind _overlappingactors (Collision|GetOverlappingActors Collision 0 :!class /Script/Engine.PrimitiveComponent))
  (bind _self self)
  (LocalVariables|SetOverlapping%20Actors _overlappingactors)
  (for _array_element _overlappingactors
    (if (not (Utilities|DoesObjectImplementInterface _array_element "/Script/GameplayAbilities.AbilitySystemInterface"))
      (Utilities|Array|RemoveItem (LocalVariables|GetOverlapping%20Actors) _array_element)))
  (Utilities|Array|RemoveItem (LocalVariables|GetOverlapping%20Actors) self)
  (Ability|SendGameplayEventtoActor _self "(TagName=\"Event.Damage\")" (Utilities|Struct|MakeGameplayEventData "(TagName=\"Event.Damage\")" _self 0 0 0 "()" "(GameplayTags=)" "(GameplayTags=)" 0.0 (Ability|TargetData|AbilityTargetDatafromActorArray (LocalVariables|GetOverlapping%20Actors)))))