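; Sparrow ability actor (AB003) that deals a one-shot area damage burst, with a particle effect and a short lifespan.
; On spawn it starts the particle system and a brief timer, then gathers actors overlapping its Sphere that implement AbilitySystemInterface.
; A CompareTeamTag macro checks each target against the instigating BP_Fighter's team tag.
; Targets that pass receive the EffectDamage gameplay effect spec from the instigator's Ability System Component.
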(event Custom|CustomEvent
  (Utilities|Time|ClearandInvalidateTimerbyHandle (stale EventBeginPlay _returnvalue))
  (CallFunction|CommitDamage (Variables|Default|GetSphere)))

(event EventBeginPlay
  (bind _returnvalue (Utilities|Time|SetTimerbyEvent (delegate Custom|CustomEvent) 0.2))
  (Components|Activation|Activate (Variables|Default|GetParticleSystem) false)
  (Actor|SetLifeSpan 2.0))

(event Collision|EventActorBeginOverlap
  (params (OtherActor :type Actor%20Object%20Reference)))

(event EventTick
  (params (DeltaSeconds :type Float%20%28single-precision%29)))

(fn ConstructionScript)

(fn CommitDamage
  (params (Collision :type Primitive%20Component%20Object%20Reference))
  (bind _overlappingactors (Collision|GetOverlappingActors Collision 0 :!class /Script/Engine.PrimitiveComponent))
  (bind _returnvalue (Game|GetInstigator))
  (LocalVariables|SetOverlapping%20Actors _overlappingactors)
  (for _array_element _overlappingactors
    (if (not (Utilities|DoesObjectImplementInterface _array_element "/Script/GameplayAbilities.AbilitySystemInterface"))
      (Utilities|Array|RemoveItem (LocalVariables|GetOverlapping%20Actors) _array_element)))
  (Utilities|Array|RemoveItem (LocalVariables|GetOverlapping%20Actors) self)
  (for _array_element_2 (LocalVariables|GetOverlapping%20Actors)
    (Utilities|CompareTeamTag _returnvalue _array_element_2
      (:else
        (GameplayEffects|ApplyGameplayEffectSpecToTarget (Ability|GetAbilitySystemComponent _returnvalue) (Variables|Default|GetEffect%20Damage) (Ability|GetAbilitySystemComponent _array_element_2))))))