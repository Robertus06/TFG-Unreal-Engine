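; Gameplay ability for Countess's standard attack, cycling through a three-montage combo across successive activations.
; After committing, it switches on AttackIndex, advances the index to the next step (wrapping after the third) and plays the matching montage.
; The ability ends when commit fails or the montage completes; other montage outcomes, such as interruption, have no handler.
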(event Ability|EventActivateAbility
  (bind _returnvalue (Ability|CommitAbility))
  (if _returnvalue
    (switch int (Variables|Default|GetAttackIndex)
      (:0
        (Variables|Default|SetAttackIndex 1)
        (|PlayMontageandWaitProxy "None" (Variables|Default|GetStandardCombo1) 1.0 "None" true 1.0 0.0 false
          (:OnCompleted
            _)))
      (:1
        (Variables|Default|SetAttackIndex 2)
        (|PlayMontageandWaitProxy "None" (Variables|Default|GetStanndardCombo2) 1.0 "None" true 1.0 0.0 false
          (:OnCompleted
            _)))
      (:2
        (Variables|Default|SetAttackIndex 0)
        (|PlayMontageandWaitProxy "None" (Variables|Default|GetStanndardCombo3) 1.0 "None" true 1.0 0.0 false
          (:OnCompleted
            _))))
    (Ability|EndAbility)
    (else
      (Ability|EndAbility))))

(event Ability|EventOnEndAbility
  (params (bWasCancelled :type Boolean)))