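; Countess character Blueprint that turns overlaps into Gameplay Ability System damage events and exposes controls for sword effects and ability hitboxes.
; Actor overlaps and SendDamage send Event.Damage to the Countess herself, with the other actor as payload target.
; Separate events toggle both sword particle systems and overlap generation on three ability colliders.
; Left and right sword overlap handlers call SendDamage, but their delegate bindings never run.
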(event Custom|OnComponentBeginOverlap_Event
  (params (OverlappedComponent :type Primitive%20Component%20Object%20Reference) (OtherActor :type Actor%20Object%20Reference) (OtherComp :type Primitive%20Component%20Object%20Reference) (OtherBodyIndex :type Integer) (bFromSweep :type Boolean) (SweepResult :type Hit%20Result%20Structure%20%28by%20ref%29))
  (CallFunction|SendDamage OtherActor))

(event Custom|SendDamage
  (params (Target :type Actor%20Object%20Reference))
  (bind _self self)
  (Ability|SendGameplayEventtoActor _self "(TagName=\"Event.Damage\")" (Utilities|Struct|MakeGameplayEventData "(TagName=\"Event.Damage\")" _self (stale Collision|EventActorBeginOverlap OtherActor))))

(event Custom|OnComponentBeginOverlap_Event_0
  (params (OverlappedComponent :type Primitive%20Component%20Object%20Reference) (OtherActor :type Actor%20Object%20Reference) (OtherComp :type Primitive%20Component%20Object%20Reference) (OtherBodyIndex :type Integer) (bFromSweep :type Boolean) (SweepResult :type Hit%20Result%20Structure%20%28by%20ref%29))
  (CallFunction|SendDamage OtherActor))

(event Custom|DeactivateSwordFX
  (Components|Activation|Deactivate (Variables|Default|GetParticleSystem1)))

(event Custom|ActivateSwordFX
  (Components|Activation|Activate (Variables|Default|GetParticleSystem1) true)
  (Components|Activation|Activate (Variables|Default|GetParticleSystem) true))

(event EventBeginPlay
  (|CallParentFunction))

(event EventEnableCollisionAbility
  (params (Ability :type EAbilities%20Enum :default "NewEnumerator0") (Enable :type Boolean))
  (switch Utilities|FlowControl|Switch|SwitchonEAbilities Ability
    (:NewEnumerator0
      (Variables|/Script/Engine.PrimitiveComponent|SetbGenerateOverlapEvents (Variables|Default|GetAbility1Coll) Enable))
    (:NewEnumerator1
      (Variables|/Script/Engine.PrimitiveComponent|SetbGenerateOverlapEvents (Variables|Default|GetAbility2Coll) Enable))
    (:NewEnumerator2
      (Variables|/Script/Engine.PrimitiveComponent|SetbGenerateOverlapEvents (Variables|Default|GetAbility3Coll) Enable))))

(event EventTick
  (params (DeltaSeconds :type Float%20%28single-precision%29))
  (|CallParentFunction DeltaSeconds) ; This node is disabled and will not be called.\nDrag off pins to build functionality.
)

(event Collision|EventActorBeginOverlap
  (params (OtherActor :type Actor%20Object%20Reference))
  (bind _self self)
  (Ability|SendGameplayEventtoActor _self "(TagName=\"Event.Damage\")" (Utilities|Struct|MakeGameplayEventData "(TagName=\"Event.Damage\")" _self OtherActor)))

(fn ConstructionScript
  (|CallParentFunction))