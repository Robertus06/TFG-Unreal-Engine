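; Khaimera's first Gameplay Ability, which deals physical damage using Gameplay Effects.
; On commit it starts a one-shot wait for Event.Damage, with the damage logic wired to the task's Then pin.
; That logic applies GE_DealDamage from payload Instigator to Target, setting SetByCaller magnitude from an Instigator attribute.
; Only a failed commit ends the ability, also removing a Countess SwordFX cue.
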(event Ability|EventActivateAbility
  (bind _returnvalue (Ability|CommitAbility))
  (if _returnvalue
    (bind _payload (Ability|Tasks|WaitGameplayEvent "(TagName=\"Event.Damage\")" 0 true)
      (:then
        (bind _returnvalue_2 (Ability|GameplayEffect|AssignTagSetbyCallerMagnitude (Ability|MakeOutgoingGameplayEffectSpec "/Game/Onyx/Effects/GE_DealDamage.GE_DealDamage_C") "(TagName=\"Data.PhysicalDamage\")" (.ReturnValue (Class|AbilitySystemComponent|GetGameplayAttributeValue (Ability|GetAbilitySystemComponent (.Instigator (Utilities|Struct|BreakGameplayEventData _payload))) "(AttributeName=\"PhysicalPower\",Attribute=/Script/Onyx.OnyxAttributeSet:PhysicalPower,AttributeOwner=\"/Script/CoreUObject.Class'/Script/Onyx.OnyxAttributeSet'\")"))))
        (GameplayEffects|ApplyGameplayEffectSpecToTarget (Ability|GetAbilitySystemComponent (.Instigator (Utilities|Struct|BreakGameplayEventData _payload))) _returnvalue_2 (Ability|GetAbilitySystemComponent (.Target (Utilities|Struct|BreakGameplayEventData _payload))))))
    (else
      (GameplayCue|RemoveGameplayCue "(TagName=\"GameplayCue.Countess.SwordFX\")")
      (Ability|EndAbility))))

(event Ability|EventOnEndAbility
  (params (bWasCancelled :type Boolean)))