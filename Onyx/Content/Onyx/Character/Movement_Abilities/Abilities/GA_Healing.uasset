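; GA_Healing is a Gameplay Ability that grants the owning fighter healing plus a timed shield.
; After committing, it notifies BP_Fighter of the ability index and cooldown through an ability-change event.
; It then applies GE_AddShield_Healing to itself, with shield amount and duration passed through SetByCaller tags, followed by GE_Healing.
; The ability ends immediately afterwards, or straight away if the commit fails, leaving the effects to run independently.
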(event Ability|EventActivateAbility
  (bind _returnvalue (Ability|CommitAbility))
  (if _returnvalue
    (Utilities|AbilityInfo 6)
    (bind _returnvalue_2 (Ability|GameplayEffect|AssignTagSetbyCallerMagnitude (Ability|MakeOutgoingGameplayEffectSpec "/Game/Onyx/Effects/GE_AddShield_Healing.GE_AddShield_Healing_C") "(TagName=\"Data.Shield\")" (Variables|Default|GetShield)))
    (bind _returnvalue_3 (Ability|GameplayEffect|AssignTagSetbyCallerMagnitude _returnvalue_2 "(TagName=\"Data.Duration\")" 1e+01))
    (GameplayEffects|ApplyGameplayEffectSpecToSelf (Ability|GetAbilitySystemComponent (Ability|GetOwningActorfromActorInfo)) _returnvalue_3)
    (GameplayEffects|ApplyGameplayEffectSpecToSelf (Ability|GetAbilitySystemComponent (Ability|GetOwningActorfromActorInfo)) (Ability|MakeOutgoingGameplayEffectSpec "/Game/Onyx/Effects/GE_Healing.GE_Healing_C"))
    (Ability|EndAbility)
    (else
      (Ability|EndAbility))))