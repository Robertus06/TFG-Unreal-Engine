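; GA_HiperDash is a gameplay ability that instantly moves the owning actor a short distance forward as a dash.
; After committing, it runs a downward-sloping visibility line trace ahead of the actor.
; It relocates the actor without sweep to just short of the hit, or to the trace end when clear; the lerp's full alpha makes this instant.
; Either outcome applies GE_HiperDash to the owner and ends the ability.
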(event Ability|EventOnEndAbility
  (params (bWasCancelled :type Boolean)))

(event Ability|EventActivateAbility
  (bind _returnvalue (Ability|GetOwningActorfromActorInfo))
  (bind _returnvalue_2 (Ability|GetOwningActorfromActorInfo))
  (bind _returnvalue_3 (Ability|MakeOutgoingGameplayEffectSpec "/Game/Onyx/Effects/GE_HiperDash.GE_HiperDash_C"))
  (bind _returnvalue_4 (Ability|GetAbilitySystemComponent _returnvalue))
  (bind _returnvalue_5 (Transformation|GetActorForwardVector _returnvalue_2))
  (bind _returnvalue_6 (Transformation|GetActorLocation _returnvalue_2))
  (bind _returnvalue_7 (+ _returnvalue_6 "0.000000,0.000000,100.000000"))
  (bind _returnvalue_8 (Ability|CommitAbility))
  (if _returnvalue_8
    (bind (_outhit _returnvalue_9) (Collision|LineTraceByChannel _returnvalue_7 (- (+ _returnvalue_6 (* _returnvalue_5 4e+02)) "0.000000,0.000000,100.000000") "TraceTypeQuery1" false 0 "None"))
    (if _returnvalue_9
      (Transformation|SetActorLocation _returnvalue (Math|Vector|Lerp(Vector) _returnvalue_7 (+ (.Location (Collision|BreakHitResult _outhit)) (* _returnvalue_5 -5e+01)) 1.0) false false)
      (GameplayEffects|ApplyGameplayEffectSpecToSelf _returnvalue_4 _returnvalue_3)
      (Ability|EndAbility)
      (else
        (Transformation|SetActorLocation _returnvalue (Math|Vector|Lerp(Vector) _returnvalue_7 (.TraceEnd (Collision|BreakHitResult _outhit)) 1.0) false false)
        (GameplayEffects|ApplyGameplayEffectSpecToSelf _returnvalue_4 _returnvalue_3)
        (Ability|EndAbility)))
    (else
      (Ability|EndAbility))))