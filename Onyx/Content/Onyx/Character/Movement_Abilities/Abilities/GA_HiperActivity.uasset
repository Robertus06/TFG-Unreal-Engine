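; GA_HiperActivity is a movement gameplay ability that boosts the owning character's speed.
; On a successful commit, it multiplies an attribute value from the owner's ability system component by SpeedInc.
; It passes the result as the Data.Speed SetByCaller magnitude on a GE_AddMovementSpeed spec applied to the owner.
; The ability ends immediately either way, leaving any duration to the effect.
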(event Ability|EventActivateAbility
  (bind _returnvalue (Ability|GetOwningActorfromActorInfo))
  (bind _returnvalue_2 (Ability|GetAbilitySystemComponent _returnvalue))
  (bind _returnvalue_3 (Ability|CommitAbility))
  (if _returnvalue_3
    (bind _returnvalue_4 (Ability|GameplayEffect|AssignTagSetbyCallerMagnitude (Ability|MakeOutgoingGameplayEffectSpec "/Game/Onyx/Effects/GE_AddMovementSpeed.GE_AddMovementSpeed_C") "(TagName=\"Data.Speed\")" (* (.ReturnValue (Class|AbilitySystemComponent|GetGameplayAttributeValue _returnvalue_2 "(AttributeName=\"MovementSpeed\",Attribute=/Script/Onyx.OnyxAttributeSet:MovementSpeed,AttributeOwner=\"/Script/CoreUObject.Class'/Script/Onyx.OnyxAttributeSet'\")")) (Variables|Default|GetSpeedInc))))
    (GameplayEffects|ApplyGameplayEffectSpecToSelf _returnvalue_2 _returnvalue_4)
    (Ability|EndAbility)
    (else
      (Ability|EndAbility))))

(event Ability|EventOnEndAbility
  (params (bWasCancelled :type Boolean)))