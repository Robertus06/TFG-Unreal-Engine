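; GA_Exhaust is a gameplay ability that slows nearby fighters and cancels their active healing.
; On a successful commit, a sphere overlap around the owner finds other BP_Fighter pawns.
; Each receives GE_ReduceMovementSpeed, with a SetByCaller magnitude scaled from an attribute of the caster, and loses effects granting the HealingActive tag.
; EndAbility runs inside the target loop or on failed commit, so an empty overlap never ends the ability.
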(event Ability|EventActivateAbility
  (bind _returnvalue (Ability|GetOwningActorfromActorInfo))
  (bind _returnvalue_2 (Ability|GetOwningActorfromActorInfo))
  (bind _returnvalue_3 (Ability|GetAbilitySystemComponent _returnvalue_2))
  (bind _returnvalue_4 (Ability|CommitAbility))
  (if _returnvalue_4
    (bind _outactors (Collision|SphereOverlapActors (Transformation|GetActorLocation _returnvalue) 5e+02 (Utilities|Array|MakeArray "ObjectTypeQuery3") "/Game/Onyx/Character/BP_Fighter.BP_Fighter_C" (Utilities|Array|MakeArray _returnvalue)))
    (for _array_element _outactors
      (bind _returnvalue_5 (Ability|GameplayEffect|AssignTagSetbyCallerMagnitude (Ability|MakeOutgoingGameplayEffectSpec "/Game/Onyx/Effects/GE_ReduceMovementSpeed.GE_ReduceMovementSpeed_C") "(TagName=\"Data.Speed\")" (* (.ReturnValue (Class|AbilitySystemComponent|GetGameplayAttributeValue _returnvalue_3 "(AttributeName=\"MovementSpeed\",Attribute=/Script/Onyx.OnyxAttributeSet:MovementSpeed,AttributeOwner=\"/Script/CoreUObject.Class'/Script/Onyx.OnyxAttributeSet'\")")) (Variables|Default|GetSpeedInc))))
      (GameplayEffects|ApplyGameplayEffectSpecToTarget _returnvalue_3 _returnvalue_5 (Ability|GetAbilitySystemComponent _array_element))
      (GameplayEffects|RemoveActiveEffectswithGrantedTags (Ability|GetAbilitySystemComponent _array_element) "(GameplayTags=((TagName=\"MovementAbilities.HealingActive\")))")
      (Ability|EndAbility))
    (else
      (Ability|EndAbility))))

(event Ability|EventOnEndAbility
  (params (bWasCancelled :type Boolean)))